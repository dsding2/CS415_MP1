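; Spawner actor that builds a chain of BP_Tunnel segments and populates them with health packs and enemies.
; On BeginPlay it destroys existing tunnels, then spawns a starting run from the player pawn's location, placing each segment at the previous one's SpawnPoint.
; Each tunnel gets a spawner back-reference, a randomized wall, a chance of a health pack and randomly scattered enemies, with spawned actors stored on that tunnel.
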(event `self.ReceiveBeginPlay`
  (`self.SpawnInitialTunnels`))

(fn `Spawn Enemies`
  (params (SpawnLocation :type "Vector Structure") (Tunnel :type "/Game/InfiniteMatrix/Blueprints/BP_Tunnel Object Reference"))
  (for _ (range (+ (`KismetMathLibrary.RandomInteger` 5) 1))
    (bind _returnvalue (`|SpawnActorFromClass` "/Game/InfiniteMatrix/Blueprints/Enemy.Enemy_C" (`KismetMathLibrary.MakeTransform` (`KismetMathLibrary.RandomPointInBoundingBox` (+ SpawnLocation (1500.0 0.0 0.0)) (500.0 200.0 200.0))) "Undefined" "MultiplyWithRoot" null null))
    (`KismetArrayLibrary.Array_Add` (`/Game/InfiniteMatrix/Blueprints/BP_Tunnel.Enemies` Tunnel) _returnvalue)))

(fn `SpawnHealthPack`
  (params (SpawnLocation :type "Vector Structure") (Tunnel :type "/Game/InfiniteMatrix/Blueprints/BP_Tunnel Object Reference"))
  (bind _returnvalue (`|SpawnActorFromClass` "/Game/InfiniteMatrix/Blueprints/HealthPack.HealthPack_C" (`KismetMathLibrary.MakeTransform` (+ SpawnLocation (`KismetMathLibrary.MakeVector` (`KismetMathLibrary.RandomFloatInRange` 500.0 2000.0) (`KismetMathLibrary.RandomFloatInRange` -200.0 200.0) (`KismetMathLibrary.RandomFloatInRange` -200.0 200.0)))) "Undefined" "MultiplyWithRoot" null null))
  (set `/Game/InfiniteMatrix/Blueprints/BP_Tunnel.HealthPack` _returnvalue Tunnel))

(fn `SpawnInitialTunnels`
  (bind _outactors (`GameplayStatics.GetAllActorsOfClass` "/Game/InfiniteMatrix/Blueprints/BP_Tunnel.BP_Tunnel_C"))
  (for _array_element _outactors
    (`self.K2_DestroyActor` _array_element))
  (for _ (range 4)
    (`/Engine/EditorBlueprintResources/StandardMacros.IsValid` (`self.NewestTunnel`)
      (:`Is Valid`
        (`self.SpawnTunnelAtSpawnPoint`))
      (:`Is Not Valid`
        (`self.SpawnTunnel` (`self.K2_GetActorLocation` (`GameplayStatics.GetPlayerPawn` 0)))))))

(fn `SpawnTunnel`
  (params (SpawnLocation :type "Vector Structure"))
  (bind _returnvalue (`|SpawnActorFromClass` "/Game/InfiniteMatrix/Blueprints/BP_Tunnel.BP_Tunnel_C" (`KismetMathLibrary.MakeTransform` SpawnLocation) "Undefined" "MultiplyWithRoot" null null))
  (bind _output_get (set `self.NewestTunnel` _returnvalue))
  (set `/Game/InfiniteMatrix/Blueprints/BP_Tunnel.TunnelSpawner` self _output_get)
  (`/Game/InfiniteMatrix/Blueprints/BP_Tunnel.RandomizeWall` _output_get)
  (`|ExecutionSequence`
    (:`then_0`
      (if (`KismetMathLibrary.RandomBoolWithWeight` 0.5)
        (`self.SpawnHealthPack` SpawnLocation _output_get)))
    (:`then_1`
      (`self.Spawn Enemies` SpawnLocation _output_get))))

(fn `SpawnTunnelAtSpawnPoint`
  (`self.SpawnTunnel` (`SceneComponent.K2_GetComponentLocation` (`/Game/InfiniteMatrix/Blueprints/BP_Tunnel.SpawnPoint` (`self.NewestTunnel`)))))

(fn `UserConstructionScript`)